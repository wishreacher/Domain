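; Base enemy character that can be stealth-killed by the player and handles its own death.
; A takedown collision flags the overlapping player as able to execute a takedown and shows a prompt widget.
; A stealth kill stops movement and plays one of eight hit-from-behind montages chosen by attack type.
; Both stealth kills and normal deaths pause mesh animation as the montage ends to hold the pose, with death also disabling collision.
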(event `self.ReceiveBeginPlay`)

(event `/Game/Character/Enemy/I_StealthKill.OnStealthKilled`
  (params (AttackType :type Integer))
  (`CharacterMovementComponent.DisableMovement` (`self.CharacterMovement`))
  (`|ExecutionSequence`
    (:`then_0`
      (`self.PlayMontages` AttackType))
    (:`then_1`
      (`KismetSystemLibrary.Delay` (- (`self.MontageDuration`) 0.05))
      (set `SkeletalMeshComponent.bPauseAnims` true (`self.Mesh`) :!label _label))))

(event `self.ProcessDeath`
  (`parent.ProcessDeath`)
  (`PrimitiveComponent.SetCollisionEnabled` (`self.CapsuleComponent`) "NoCollision")
  (`PrimitiveComponent.SetCollisionEnabled` (`self.TakeDownCollision`) "NoCollision")
  (`KismetSystemLibrary.Delay` (`AnimSequenceBase.SequenceLength` (`self.OnDeathAnimMontage`)))
  (goto _label))

(event `self.TakeDownCollision.OnComponentBeginOverlap`
  (params (OverlappedComponent :type "PrimitiveComponent Object Reference") (OtherActor :type "Actor Object Reference") (OtherComp :type "PrimitiveComponent Object Reference") (OtherBodyIndex :type Integer) (bFromSweep :type Boolean) (SweepResult :type "HitResult Structure (by ref)"))
  (bind _asbp_player (cast `/Game/Character/Player/BP_Player` OtherActor))
  (set `/Game/Character/Player/BP_Player.CanExecuteTakedown` true _asbp_player)
  (bind _returnvalue (`|CreateWidget` "/Game/UI/W_CanExecuteTakedown.W_CanExecuteTakedown_C"))
  (bind _output_get (set `self.TakedownWidget` _returnvalue))
  (`UserWidget.AddToViewport` _output_get 0))

(event `self.TakeDownCollision.OnComponentEndOverlap`
  (params (OverlappedComponent :type "PrimitiveComponent Object Reference") (OtherActor :type "Actor Object Reference") (OtherComp :type "PrimitiveComponent Object Reference") (OtherBodyIndex :type Integer))
  (bind _asbp_player (cast `/Game/Character/Player/BP_Player` OtherActor))
  (set `/Game/Character/Player/BP_Player.CanExecuteTakedown` false _asbp_player)
  (`Widget.RemoveFromParent` (`self.TakedownWidget`)))

(fn `CanTakedown`
  (returns (return :type Boolean))
  (return (`self.CanBeTakenDown`)))

(fn `PlayMontages`
  (params (Selection :type Integer))
  (switch `int` Selection
    (:`0`
      (bind _returnvalue (`self.PlayAnimMontage` "/Game/Character/Player/Animations/Stealth/Hit/AM_Stealth_Kill_Hit_Behind_01.AM_Stealth_Kill_Hit_Behind_01"))
      (set `self.MontageDuration` _returnvalue))
    (:`1`
      (bind _returnvalue_2 (`self.PlayAnimMontage` "/Game/Character/Player/Animations/Stealth/Hit/AM_Stealth_Kill_Hit_Behind_02.AM_Stealth_Kill_Hit_Behind_02"))
      (set `self.MontageDuration` _returnvalue_2))
    (:`2`
      (bind _returnvalue_3 (`self.PlayAnimMontage` "/Game/Character/Player/Animations/Stealth/Hit/AM_Stealth_Kill_Hit_Behind_03.AM_Stealth_Kill_Hit_Behind_03"))
      (set `self.MontageDuration` _returnvalue_3))
    (:`3`
      (bind _returnvalue_4 (`self.PlayAnimMontage` "/Game/Character/Player/Animations/Stealth/Hit/AM_Stealth_Kill_Hit_Behind_04.AM_Stealth_Kill_Hit_Behind_04"))
      (set `self.MontageDuration` _returnvalue_4))
    (:`4`
      (bind _returnvalue_5 (`self.PlayAnimMontage` "/Game/Character/Player/Animations/Stealth/Hit/AM_Stealth_Kill_Hit_Behind_05.AM_Stealth_Kill_Hit_Behind_05"))
      (set `self.MontageDuration` _returnvalue_5))
    (:`5`
      (bind _returnvalue_6 (`self.PlayAnimMontage` "/Game/Character/Player/Animations/Stealth/Hit/AM_Stealth_Kill_Hit_Behind_06.AM_Stealth_Kill_Hit_Behind_06"))
      (set `self.MontageDuration` _returnvalue_6))
    (:`6`
      (bind _returnvalue_7 (`self.PlayAnimMontage` "/Game/Character/Player/Animations/Stealth/Hit/AM_Stealth_Kill_Hit_Behind_07.AM_Stealth_Kill_Hit_Behind_07"))
      (set `self.MontageDuration` _returnvalue_7))
    (:`7`
      (bind _returnvalue_8 (`self.PlayAnimMontage` "/Game/Character/Player/Animations/Stealth/Hit/AM_Stealth_Kill_Hit_Behind_08.AM_Stealth_Kill_Hit_Behind_08"))
      (set `self.MontageDuration` _returnvalue_8))))

(fn `UserConstructionScript`)