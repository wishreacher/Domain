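; Player component that runs stealth takedowns on enemies, from finding the target to cleaning up afterwards.
; A forward pawn trace sets the behind-takedown target, and the player capsule moves to an offset in the target's local axes, matching its rotation.
; The takedown data supplies the player montage, weapon socket and a temporary tracking camera rig.
; Ending the takedown destroys the rig and restores the melee weapon's socket.
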(event `self.ReceiveBeginPlay`
  (bind _asbp_player (cast `/Game/Character/Player/BP_Player` (`GameplayStatics.GetPlayerCharacter` 0)))
  (set `self.CharacterRef` _asbp_player))

(event `self.TakeDownCameraRigActivation`
  (params (TakeDown :type "TakeDownDescription Structure"))
  (bind _characterref (`self.CharacterRef`))
  (bind _characterref_2 (`self.CharacterRef`))
  (bind _bpc_camerarig (`/Game/Character/Player/BP_Player.BPC_CameraRig` _characterref))
  (bind _bpc_camerarig_2 (`/Game/Character/Player/BP_Player.BPC_CameraRig` _characterref_2))
  (set `/Game/Character/Player/BP_Player.CurrentTakeDownCount` 0 (`self.CharacterRef`))
  (bind _asbp_camera_rig_base (castclass `/Game/PluginAssets/CameraRig/Blueprint/Rigs/Base/BP_CameraRig_Base` TakeDown_CameraMovement))
  (bind (_created_ _camerarig) (`/Game/PluginAssets/CameraRig/Blueprint/Components/BPC_CameraRig.CreateCameraRig` _bpc_camerarig_2 _asbp_camera_rig_base (`Actor.GetTransform` _characterref_2) "TakeDown"))
  (if _created_
    (bind _currentswitchsettings_newspottype (break `/Game/PluginAssets/CameraRig/Structs/S_CameraSwitchSettings` (`/Game/PluginAssets/CameraRig/Blueprint/Components/BPC_CameraRig.GetSwitchSettings` _bpc_camerarig_2 _camerarig)))
    (`/Game/PluginAssets/CameraRig/Blueprint/Components/BPC_CameraRig.TriggerCameraRigByRef` _bpc_camerarig _camerarig _currentswitchsettings_newspottype 0)
    (`/Game/PluginAssets/CameraRig/Blueprint/Components/BPC_CameraRig.UpdateTrackingActor` _bpc_camerarig true (`|ConvertAsset` (`/Game/Character/Player/BP_Player.PointToTrack` _characterref)) (0.0 0.0 0.0) false 0.0)
    (set `/Game/Character/Player/BP_Player.CreatedTakeDownRig` _camerarig _characterref)))

(event `self.EnemyTakeDownInterfaceCall`
  (params (Target :type "Actor Object Reference") (TakeDown :type "TakeDownDescription Structure"))
  (message `/Game/Character/Enemy/I_StealthKill.OnStealthKilled` Target TakeDown))

(event `self.PlayTakeDownMontages`
  (params (TakeDownDescription :type "TakeDownDescription Structure"))
  (`self.Play Take Down Monatges` TakeDownDescription))

(event `self.TakeDownEnd`
  (bind _characterref (`self.CharacterRef`))
  (bind _characterref_2 (`self.CharacterRef`))
  (bind _returnvalue (`CharacterEquipmentComponent.GetCurrentMeleeWeapon` (`BaseCharacter.CharacterEquipmentComponent` _characterref_2)))
  (`parent.TakeDownEnd`)
  (`/Game/PluginAssets/CameraRig/Blueprint/Components/BPC_CameraRig.DestroyCameraRigByRef` (`/Game/Character/Player/BP_Player.BPC_CameraRig` _characterref) (`/Game/Character/Player/BP_Player.CreatedTakeDownRig` _characterref) "TakeDown")
  (`/Engine/EditorBlueprintResources/StandardMacros.IsValid` _returnvalue
    (:`Is Valid`
      (`Actor.K2_AttachToComponent` _returnvalue (`Character.Mesh` _characterref_2) (`EquippableItem.EquippedSocketName` _returnvalue) "SnapToTarget" "SnapToTarget" "SnapToTarget" true))))

(event `self.MoveToTakeDownTarget`
  (params (TargetActor :type "Actor Object Reference") (Offset :type "Vector Structure"))
  (bind _returnvalue (`self.TakeDownOffsetCalculation` TargetActor Offset))
  (`KismetSystemLibrary.MoveComponentTo` (`Character.CapsuleComponent` (`self.CharacterRef`)) _returnvalue (`Actor.K2_GetActorRotation` TargetActor)))

(event `self.SetupTarget`
  (bind _characterref (`self.CharacterRef`))
  (bind _returnvalue (`Actor.K2_GetActorLocation` (`self.CharacterRef`)))
  (bind (_outhit _returnvalue_2) (`KismetSystemLibrary.LineTraceSingleForObjects` _returnvalue (+ _returnvalue (* (`/Game/Character/Player/BP_Player.TakedownRange` _characterref) (`Actor.GetActorForwardVector` _characterref))) (`|MakeArray` "ObjectTypeQuery3" :!type "EObjectTypeQuery Enum")))
  (if _returnvalue_2
    (`self.SetBehindTakeDownTarget` (`.HitActor` (`GameplayStatics.BreakHitResult` _outhit)))))

(fn `Play Take Down Monatges`
  (params (Description :type "TakeDownDescription Structure"))
  (bind _characterref (`self.CharacterRef`))
  (bind _returnvalue (`CharacterEquipmentComponent.GetCurrentMeleeWeapon` (`BaseCharacter.CharacterEquipmentComponent` _characterref)))
  (bind _returnvalue_2 (`Character.PlayAnimMontage` _characterref Description_PlayerTakeDownMontage 1.0 "None"))
  (set `/Game/Character/Player/BP_Player.MontageDuration` _returnvalue_2 _characterref)
  (`/Engine/EditorBlueprintResources/StandardMacros.IsValid` _returnvalue
    (:`Is Valid`
      (`Actor.K2_AttachToComponent` _returnvalue (`Character.Mesh` _characterref) Description_EquippedSocketName "SnapToTarget" "SnapToTarget" "SnapToTarget" true))))

(fn `TakeDownOffsetCalculation`
  (params (TargetActor :type "Actor Object Reference") (Offset :type "Vector Structure"))
  (returns (ReturnValue :type "Vector Structure"))
  (return (- (- (- (`Actor.K2_GetActorLocation` TargetActor) (* (`Actor.GetActorForwardVector` TargetActor) (`KismetSystemLibrary.MakeLiteralDouble` Offset_X))) (* (`Actor.GetActorRightVector` TargetActor) (`KismetSystemLibrary.MakeLiteralDouble` Offset_Y))) (* (`Actor.GetActorUpVector` TargetActor) (`KismetSystemLibrary.MakeLiteralDouble` Offset_Z)))))