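; Player character Blueprint handling camera behavior and enemy lock-on.
; Timelines drive sprint arm length and aim FOV, a spawned pelvis-attached actor serves camera rigs, and the equipped slot sets rotation mode.
; While unlocked, Tick box-traces along the view for enemies; lock-on targets the nearest, turning actor and controller toward it.
; Lock-on works only unarmed or with melee, using visibility traces, a release timer and a range limit to drop targets.
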(event `self.SetAimCameraFOV`
  (bind (_direction _newtrack_0) (`Timeline|AimCameraFOV` :!via `PlayFromStart` :!label _label)
    (:`Update`
      (`CameraComponent.SetFieldOfView` (`self.CameraComponent`) (`KismetMathLibrary.Lerp` (`CameraComponent.FieldOfView` (`self.CameraComponent`)) (`RangeWeapon.GetAimFOV` (`CharacterEquipmentComponent.GetCurrentRangeWeapon` (`self.CharacterEquipmentComponent`))) _newtrack_0)))))

(event `self.ReceiveBeginPlay`
  (set `self.DefaultArmLenght` (`SpringArmComponent.TargetArmLength` (`self.SpringArmComponent`)))
  ;[1 1 1] Setting up an actor to track in camera rigs
  (bind _returnvalue (`|SpawnActorFromClass` "/Game/Weapons/SingleDagger/CameraRigs/BP_FocusTarget.BP_FocusTarget_C" (`self.GetTransform`) "Undefined" "OverrideRootScale" null null))
  (`self.K2_AttachToComponent` _returnvalue (`self.Mesh`) "pelvisSocket" "SnapToTarget" "SnapToTarget" "SnapToTarget" true)
  (set `self.PointToTrack` _returnvalue))

(event `self.SetDefaultCameraFOV`
  (`|ExecutionSequence`
    (:`then_0`
      (goto _label :!via `Stop`))
    (:`then_1`
      (`CameraComponent.SetFieldOfView` (`self.CameraComponent`) 90.0))))

(event `self.OnSprintStart`
  ;[1 1 1] Sprint Arm
  (bind (_direction _newtrack_0) (`Timeline|Timeline_0` :!label _label_2)
    (:`Update`
      (set `SpringArmComponent.TargetArmLength` (`KismetMathLibrary.Lerp` (`self.DefaultArmLenght`) (`self.SprintArmLenght`) _newtrack_0) (`self.SpringArmComponent`)))))

(event `self.OnSprintEnd`
  ;[1 1 1] Sprint Arm
  (goto _label_2 :!via `Reverse`))

(event `RemoveLockOn`
  (`self.ToggleLockOn` false))

(event `self.ReceiveTick`
  (params (DeltaSeconds :type "Float (single-precision)"))
  (bind _returnvalue (`self.GetController`))
  (bind (_returnvalue_roll _returnvalue_pitch) (`KismetMathLibrary.BreakRotator` (`self.K2_GetActorRotation`)))
  (bind _istargetvisibletimerhandle (`self.IsTargetVisibleTimerHandle`))
  (bind _basecharactermovementcomponent (`self.BaseCharacterMovementComponent`))
  (bind _returnvalue_2 (`Controller.GetControlRotation` _returnvalue))
  (bind (_returnvalue_roll_2 _returnvalue_pitch_2 _returnvalue_yaw) (`KismetMathLibrary.BreakRotator` (`KismetMathLibrary.RInterpTo` (`KismetMathLibrary.FindLookAtRotation` (`self.K2_GetActorLocation`) (`self.K2_GetActorLocation` (`self.LockedOnEnemy`))) (`self.K2_GetActorRotation`) (`GameplayStatics.GetWorldDeltaSeconds`) 20.0)))
  (bind _visibleactors (`self.TraceForEnemies`))
  (if (`self.ShouldCameraFocusEnemy`)
    (`self.ToggleLockOn` true)
    (switch `EEquipmentSlots` (`CharacterEquipmentComponent.GetCurrentEquippedSlot` (`self.CharacterEquipmentComponent`))
      (:`None`
        (bind _output_get (set `self.LockedOnEnemy` (`.ReturnValue` (`GameplayStatics.FindNearestActor` (`self.K2_GetActorLocation`) _visibleactors)) :!label _label_3))
        (bind _outhit (`KismetSystemLibrary.LineTraceSingle` (`Controller.GetPlayerViewPoint` (`GameplayStatics.GetPlayerController` 0)) (`self.K2_GetActorLocation` (`self.LockedOnEnemy`)) "TraceTypeQuery5"))
        (bind (_bblockinghit _binitialoverlap _time _distance _location _impactpoint _normal _impactnormal _physmat _hitactor) (`GameplayStatics.BreakHitResult` _outhit))
        (if (and _bblockinghit (== (`self.LockedOnEnemy`) _hitactor))
          (`|ExecutionSequence`
            (:`then_0`
              (goto _label_6 :!via `Reset`))
            (:`then_1`
              (if (`KismetSystemLibrary.K2_IsValidTimerHandle` _istargetvisibletimerhandle)
                (`KismetSystemLibrary.K2_ClearAndInvalidateTimerHandle` _istargetvisibletimerhandle))
              (if (> (`self.GetDistanceTo` (`self.LockedOnEnemy`)) 10000.0)
                (`self.ToggleLockOn` false)
                (else
                  (`/Engine/EditorBlueprintResources/StandardMacros.IsValid` _output_get
                    (:`Is Valid`
                      (`self.K2_SetActorRotation` (`KismetMathLibrary.MakeRotator` _returnvalue_roll _returnvalue_pitch _returnvalue_yaw))
                      (`Controller.SetControlRotation` _returnvalue (`KismetMathLibrary.MakeRotator` (.roll _returnvalue_2) (.pitch _returnvalue_2) (.yaw (`KismetMathLibrary.RInterpTo` _returnvalue_2 (`KismetMathLibrary.FindLookAtRotation` (`SceneComponent.K2_GetComponentLocation` (`self.CameraComponent`)) (`self.K2_GetActorLocation` (`self.LockedOnEnemy`))) (`GameplayStatics.GetWorldDeltaSeconds`) 5.0))))
                      (switch `EEquipmentSlots` (`CharacterEquipmentComponent.GetCurrentEquippedSlot` (`self.CharacterEquipmentComponent`)) :!label _label_4
                        (:`None`
                          (set `self.bUseControllerRotationYaw` false)
                          (set `CharacterMovementComponent.bOrientRotationToMovement` true _basecharactermovementcomponent))
                        (:`SideArm`
                          (set `self.bUseControllerRotationYaw` true :!label _label_5)
                          (set `CharacterMovementComponent.bOrientRotationToMovement` false _basecharactermovementcomponent))
                        (:`PrimaryWeapon`
                          (goto _label_5))
                        (:`SecondaryWeapon`
                          (goto _label_5))
                        (:`MeleeWeapon`
                          (goto _label_5))))
                    (:`Is Not Valid`
                      (`self.ToggleLockOn` false)))))))
          (else
            (`/Engine/EditorBlueprintResources/StandardMacros.DoOnce` false :!label _label_6
              (:`Completed`
                (bind _returnvalue_3 (`KismetSystemLibrary.K2_SetTimerDelegate` (delegate `RemoveLockOn`) 3.0))
                (set `self.IsTargetVisibleTimerHandle` _returnvalue_3))))))
      (:`SideArm`
        (`self.ToggleLockOn` false :!label _label_7))
      (:`PrimaryWeapon`
        (goto _label_7))
      (:`SecondaryWeapon`
        (goto _label_7))
      (:`MeleeWeapon`
        (goto _label_3)))
    (else
      (goto _label_4))))

(event `InputAction|LockOn`
  (params (Key :type "Key Structure"))
  (:`Pressed`
    (`self.ToggleLockOn` (not (`self.ShouldCameraFocusEnemy`)))))

(event `ToggleLockOn`
  (params (`Is Lock` :type Boolean))
  (set `self.ShouldCameraFocusEnemy` `Is Lock`)
  (set `CharacterMovementComponent.bOrientRotationToMovement` (not `Is Lock`) (`self.BaseCharacterMovementComponent`))
  (if `Is Lock`
    (message `/Game/Character/Enemy/I_EnemyInteraction.AddTarget` (`self.LockedOnEnemy`))
    (else
      (message `/Game/Character/Enemy/I_EnemyInteraction.RemoveTarget` (`self.LockedOnEnemy`))
      (set `self.LockedOnEnemy` null))))

(fn `CanTakedown`
  (returns (return :type Boolean))
  (return false))

(fn `TraceForEnemies`
  (returns (VisibleActors :type "Array of Actor Object Reference"))
  (bind _returnvalue (`self.K2_GetActorLocation`))
  (bind (_location _rotation) (`Controller.GetPlayerViewPoint` (`GameplayStatics.GetPlayerController` 0)))
  (if (not (`self.ShouldCameraFocusEnemy`))
    (`KismetArrayLibrary.Array_Clear` (`self.VisibleActors`))
    (bind (_outhits _returnvalue_2) (`KismetSystemLibrary.BoxTraceMultiForObjects` (+ _returnvalue (* (`self.GetActorForwardVector`) 100.0)) (+ _returnvalue (* 10000.0 _rotation)) (20.0 120.0 20.0) _rotation (`|MakeArray` "ObjectTypeQuery3" :!type "EObjectTypeQuery Enum")))
    (if _returnvalue_2
      (for _array_element _outhits
        (bind (_bblockinghit _binitialoverlap _time _distance _location_2 _impactpoint _normal _impactnormal _physmat _hitactor) (`GameplayStatics.BreakHitResult` _array_element))
        (if (`KismetMathLibrary.ClassIsChildOf` (`GameplayStatics.GetObjectClass` _hitactor) "/Script/Domain.EnemyCharacter")
          (`KismetArrayLibrary.Array_AddUnique` (`self.VisibleActors`) _hitactor)))
      (return (`self.VisibleActors`)))))

(fn `TriggerRigWithNumber`
  (params (TriggerSpot_Index :type Integer) (CameraRig :type "/Game/PluginAssets/CameraRig/Blueprint/Rigs/Base/BP_CameraRig_Base Object Reference"))
  (`/Game/PluginAssets/CameraRig/Blueprint/Components/BPC_CameraRig.TriggerCameraRigByRef` (`self.BPC_CameraRig`) CameraRig "NewEnumerator0" TriggerSpot_Index))

(fn `UserConstructionScript`)