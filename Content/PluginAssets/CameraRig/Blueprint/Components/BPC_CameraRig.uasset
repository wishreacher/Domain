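; Manager component for cine camera rigs that spawns, triggers, switches, exits and destroys BP_CameraRig_Base actors.
; On BeginPlay it registers every rig in the level by reference and name, then applies the debug mode, with an optional HUD widget.
; It tracks the current rig and delegates camera work to it.
; It also holds global focus and look-at settings, forwards per-rig settings, and refreshes all rigs when global tracking changes.
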(event `self.ReceiveBeginPlay`
  (`self.GetAllRigsInLevel`)
  (`self.Debug` (`self.DebugMode`) (`self.Debug_TraceDuration`)))

(fn `CanChangeRig?`
  (returns (ReturnValue :type Boolean))
  (return (not (`self.OnRigChanging?`))))

(fn `ChangeRig`
  (params (NewCameraRig :type "/Game/PluginAssets/CameraRig/Blueprint/Rigs/Base/BP_CameraRig_Base Object Reference") (RigChange_Settings :type "/Game/PluginAssets/CameraRig/Structs/S_CameraSwitchSettings Structure") (`DestroyOldRig?` :type Boolean))
  (`/Engine/EditorBlueprintResources/StandardMacros.IsValid` NewCameraRig
    (:`Is Valid`
      (`/Engine/EditorBlueprintResources/StandardMacros.IsValid` (`self.GetCurrentCameraRig`)
        (:`Is Valid`
          (if (!= (`self.GetCurrentCameraRig`) NewCameraRig)
            (`/Game/PluginAssets/CameraRig/Blueprint/Rigs/Base/BP_CameraRig_Base.CE_ChangeToRig` (`self.GetCurrentCameraRig`) NewCameraRig RigChange_Settings `DestroyOldRig?`)
            (`self.SetCurrentCameraRig` NewCameraRig)
            (else
              (`self.PrintString_Debug` "NewEnumerator1" "CameraRig: \n \nCant change rig \n \nCurrent and new rig are the same"))))))))

(fn `CreateCameraRig`
  (params (CameraRig_Class :type "/Game/PluginAssets/CameraRig/Blueprint/Rigs/Base/BP_CameraRig_Base Class Reference") (SpawnTransform :type "Transform Structure") (`Rigname/ID` :type Text))
  (returns (`Created?` :type Boolean) (CameraRig :type "/Game/PluginAssets/CameraRig/Blueprint/Rigs/Base/BP_CameraRig_Base Object Reference"))
  (locals (L_CameraRigClass :type "/Game/PluginAssets/CameraRig/Blueprint/Rigs/Base/BP_CameraRig_Base Class Reference") (L_SpawnTransform :type "Transform Structure") (L_Rigname :type Text))
  (set `local.L_CameraRigClass` CameraRig_Class)
  (set `local.L_SpawnTransform` SpawnTransform)
  (set `local.L_Rigname` `Rigname/ID`)
  (if (`KismetArrayLibrary.Array_Contains` (`self.CameraRigNames`) (`local.L_Rigname`))
    (`self.PrintString_Debug` "NewEnumerator1" (`KismetStringLibrary.Concat_StrStr` "Cant create rig! \n \nName is already taken. \n" "Name: " (`KismetTextLibrary.Conv_TextToString` (`local.L_Rigname`))))
    (return false null)
    (else
      (bind _returnvalue (`|SpawnActorFromClass` (`local.L_CameraRigClass`) (`local.L_SpawnTransform`) "AlwaysSpawn" "OverrideRootScale" null self (`local.L_Rigname`) null))
      (`KismetArrayLibrary.Array_AddUnique` (`self.CameraRigs`) _returnvalue)
      (`KismetArrayLibrary.Array_AddUnique` (`self.CameraRigNames`) (`local.L_Rigname`))
      (`self.Debug` (`self.DebugMode`) (`self.Debug_TraceDuration`))
      (return true _returnvalue))))

(fn `CreateDebugWidget`
  (returns (DebugWidget :type "/Game/PluginAssets/CameraRig/Widgets/WB_CameraHud Object Reference"))
  (bind _returnvalue (`|CreateWidget` "/Game/PluginAssets/CameraRig/Widgets/WB_CameraHud.WB_CameraHud_C"))
  (`UserWidget.AddToViewport` _returnvalue 0)
  (bind _output_get (set `self.WB_CameraHud` _returnvalue))
  (return _output_get))

(fn `Debug`
  (params (`Debug Type` :type "/Game/PluginAssets/CameraRig/Enums/E_Camspot_DebugModes Enum" :default "NewEnumerator0") (TraceDuration :type "Float (double-precision)"))
  (locals (L_TraceDuration :type "Float (double-precision)"))
  (set `local.L_TraceDuration` TraceDuration)
  (setmembers `CameraLookatTrackingSettings` :`StructRef` (`self.Global_LookatTrackingSettings`) :`bDrawDebugLookAtTrackingPosition` (select `/Game/PluginAssets/CameraRig/Enums/E_Camspot_DebugModes` `Debug Type` :`NewEnumerator2` true :`NewEnumerator3` true))
  (for _array_element (`self.CameraRigs`)
    (set `/Game/PluginAssets/CameraRig/Blueprint/Rigs/Base/BP_CameraRig_Base.Debug_Trace` (`self.Debug_TraceDuration`) _array_element)
    (set `/Game/PluginAssets/CameraRig/Blueprint/Rigs/Base/BP_CameraRig_Base.DebugMode?` `Debug Type` _array_element)
    (`/Game/PluginAssets/CameraRig/Blueprint/Rigs/Base/BP_CameraRig_Base.StartDebugTimer` _array_element))
  (switch `/Game/PluginAssets/CameraRig/Enums/E_Camspot_DebugModes` (`local.Debug Type`)
    (:`NewEnumerator1`
      _)
    (:`NewEnumerator3`
      _))
  (`self.CreateDebugWidget`))

(fn `DestroyCameraRigByRef`
  (params (CameraRig :type "/Game/PluginAssets/CameraRig/Blueprint/Rigs/Base/BP_CameraRig_Base Object Reference") (`Camera Rig Name` :type Text))
  (locals (L_CameraRig :type "/Game/PluginAssets/CameraRig/Blueprint/Rigs/Base/BP_CameraRig_Base Object Reference"))
  (set `local.L_CameraRig` CameraRig)
  (`KismetArrayLibrary.Array_RemoveItem` (`self.CameraRigs`) (`local.L_CameraRig`))
  (`KismetArrayLibrary.Array_RemoveItem` (`self.CameraRigNames`) `Camera Rig Name`)
  (`/Engine/EditorBlueprintResources/StandardMacros.IsValid` (`/Game/PluginAssets/CameraRig/Blueprint/Rigs/Base/BP_CameraRig_Base.CineCamera` (`local.L_CameraRig`))
    (:`Is Valid`
      (`Actor.K2_DestroyActor` (`/Game/PluginAssets/CameraRig/Blueprint/Rigs/Base/BP_CameraRig_Base.CineCamera` (`local.L_CameraRig`))))
    (:`Is Not Valid`
      _))
  (`Actor.K2_DestroyActor` (`local.L_CameraRig`))
  (return))

(fn `DetroyCameraRigByName`
  (params (CameraRigName :type Text))
  (returns (`Success?` :type Boolean))
  (bind (_found_ _camerarig) (`self.GetCameraRigByName` CameraRigName))
  (if _found_
    (`self.DestroyCameraRigByRef` _camerarig CameraRigName)
    (return true)
    (else
      (return false))))

(fn `GetAllCameraRigNames`
  (returns (RigNames :type "Array of Text"))
  (locals (L_RigNames :type "Array of Text"))
  (return (`local.L_RigNames`)))

(fn `GetAllCameraRigRefs`
  (returns (CameraRigs :type "Array of /Game/PluginAssets/CameraRig/Blueprint/Rigs/Base/BP_CameraRig_Base Object Reference"))
  (return (`self.CameraRigs`)))

(fn `GetAllRigSettings`
  (params (CameraRig :type "/Game/PluginAssets/CameraRig/Blueprint/Rigs/Base/BP_CameraRig_Base Object Reference"))
  (returns (CameraRail_Settings :type "/Game/PluginAssets/CameraRig/Structs/S_CameraRail_Settings Structure") (CurrentSwitchSettings :type "/Game/PluginAssets/CameraRig/Structs/S_CameraSwitchSettings Structure") (`Focus Settings` :type "/Game/PluginAssets/CameraRig/Structs/S_CameraRig_FocusSettings Structure") (`Lookat Tracking Settings` :type "CameraLookatTrackingSettings Structure"))
  (return (`self.GetRailSettings` CameraRig) (`self.GetSwitchSettings` CameraRig) (`self.GetLocalFocusSettings` CameraRig) (`self.GetLocalTrackingSettings` CameraRig)))

(fn `GetAllRigsInLevel`
  (bind _outactors (`GameplayStatics.GetAllActorsOfClass` "/Game/PluginAssets/CameraRig/Blueprint/Rigs/Base/BP_CameraRig_Base.BP_CameraRig_Base_C"))
  (for (_array_element _array_index) _outactors
    (`KismetArrayLibrary.Array_AddUnique` (`self.CameraRigs`) _array_element)
    (bind _rigname (`/Game/PluginAssets/CameraRig/Blueprint/Rigs/Base/BP_CameraRig_Base.Rigname` _array_element))
    (`KismetArrayLibrary.Array_AddUnique` (`self.CameraRigNames`) (select `bool` (`KismetTextLibrary.EqualEqual_TextText` _rigname "") :`false` _rigname :`true` (`KismetTextLibrary.Conv_StringToText` (`KismetStringLibrary.Concat_StrStr` "NoName" (`KismetStringLibrary.Conv_IntToString` _array_index))))))
  (return))

(fn `GetCameraRigByName`
  (params (CameraRigName :type Text))
  (returns (`Found?` :type Boolean) (CameraRig :type "/Game/PluginAssets/CameraRig/Blueprint/Rigs/Base/BP_CameraRig_Base Object Reference"))
  (locals (L_CameraRigName :type Text) (`L_Found?` :type Boolean :default false) (L_FoundRig :type "/Game/PluginAssets/CameraRig/Blueprint/Rigs/Base/BP_CameraRig_Base Object Reference"))
  (set `local.L_CameraRigName` CameraRigName)
  (for _array_element (`self.CameraRigs`)
    (if (`KismetTextLibrary.EqualEqual_TextText` (`/Game/PluginAssets/CameraRig/Blueprint/Rigs/Base/BP_CameraRig_Base.Rigname` _array_element) (`local.L_CameraRigName`))
      (set `local.L_FoundRig` _array_element)
      (set `local.L_Found?` true)
      (break)))
  (return (`local.L_Found?`) (`local.L_FoundRig`)))

(fn `GetCurrentCameraRig`
  (returns (CurrentCameraRig :type "/Game/PluginAssets/CameraRig/Blueprint/Rigs/Base/BP_CameraRig_Base Object Reference"))
  (return (`self.CurrentCameraRig`)))

(fn `GetGlobalFocusSettings`
  (returns (GlobalFocusSettings :type "/Game/PluginAssets/CameraRig/Structs/S_CameraRig_FocusSettings Structure"))
  (return (`self.Global_FocusSettings`)))

(fn `GetGlobalTrackingSettings`
  (returns (Global_LookatTrackingSettings :type "CameraLookatTrackingSettings Structure"))
  (return (`self.Global_LookatTrackingSettings`)))

(fn `GetLocalFocusSettings`
  (params (CameraRig :type "/Game/PluginAssets/CameraRig/Blueprint/Rigs/Base/BP_CameraRig_Base Object Reference"))
  (returns (`Focus Settings` :type "/Game/PluginAssets/CameraRig/Structs/S_CameraRig_FocusSettings Structure"))
  (return (`/Game/PluginAssets/CameraRig/Blueprint/Rigs/Base/BP_CameraRig_Base.LocalFocusSettings` CameraRig)))

(fn `GetLocalTrackingSettings`
  (params (CameraRig :type "/Game/PluginAssets/CameraRig/Blueprint/Rigs/Base/BP_CameraRig_Base Object Reference"))
  (returns (`Lookat Tracking Settings` :type "CameraLookatTrackingSettings Structure"))
  (return (`/Game/PluginAssets/CameraRig/Blueprint/Rigs/Base/BP_CameraRig_Base.LocalLookatTrackingSettings` CameraRig)))

(fn `GetRailSettings`
  (params (CameraRig :type "/Game/PluginAssets/CameraRig/Blueprint/Rigs/Base/BP_CameraRig_Base Object Reference"))
  (returns (CameraRail_Settings :type "/Game/PluginAssets/CameraRig/Structs/S_CameraRail_Settings Structure"))
  (locals (L_CameraRig :type "/Game/PluginAssets/CameraRig/Blueprint/Rigs/Base/BP_CameraRig_Base Object Reference"))
  (set `local.L_CameraRig` CameraRig)
  (`/Engine/EditorBlueprintResources/StandardMacros.IsValid` (`local.L_CameraRig`)
    (:`Is Valid`
      (return (`/Game/PluginAssets/CameraRig/Blueprint/Rigs/Base/BP_CameraRig_Base.GetRailSettings` (`local.L_CameraRig`))))))

(fn `GetSwitchSettings`
  (params (CameraRig :type "/Game/PluginAssets/CameraRig/Blueprint/Rigs/Base/BP_CameraRig_Base Object Reference"))
  (returns (CurrentSwitchSettings :type "/Game/PluginAssets/CameraRig/Structs/S_CameraSwitchSettings Structure"))
  (locals (L_CameraRig :type "/Game/PluginAssets/CameraRig/Blueprint/Rigs/Base/BP_CameraRig_Base Object Reference"))
  (set `local.L_CameraRig` CameraRig)
  (`/Engine/EditorBlueprintResources/StandardMacros.IsValid` (`local.L_CameraRig`)
    (:`Is Valid`
      (return (`/Game/PluginAssets/CameraRig/Blueprint/Rigs/Base/BP_CameraRig_Base.GetSwitchSettings` (`local.L_CameraRig`))))))

(fn `LeaveRig`
  (params (BlendTime :type "Float (double-precision)") (BlendFunc :type "EViewTargetBlendFunction Enum" :default "VTBlend_Linear"))
  (locals (`L_DestroyRig?` :type Boolean) (L_BlendTime :type "Float (double-precision)"))
  (set `local.L_BlendTime` BlendTime)
  (`self.CurrentCameraRig`
    (:`then`
      (`/Game/PluginAssets/CameraRig/Blueprint/Rigs/Base/BP_CameraRig_Base.CE_Exit_CameraRig` (`self.CurrentCameraRig`) BlendTime BlendFunc)
      (`self.SetCurrentCameraRig` null))
    (:`else`)))

(fn `PrintString_Debug`
  (params (PrintType :type "/Game/PluginAssets/CameraRig/Enums/E_Camspot_DebugPrint Enum" :default "NewEnumerator0") (Message :type String))
  (`KismetSystemLibrary.PrintString` (`KismetStringLibrary.Concat_StrStr` (`|GetEnumeratorNameAsString` PrintType) ": \n" Message) true true (select `/Game/PluginAssets/CameraRig/Enums/E_Camspot_DebugPrint` PrintType :`NewEnumerator0` (struct :`G` 0.380107 :`B` 1.0 :`A` 1.0) :`NewEnumerator1` (struct :`R` 1.0 :`G` 0.825233 :`A` 1.0) :`NewEnumerator2` (struct :`R` 1.0 :`B` 0.052352 :`A` 1.0) :!type "LinearColor Structure") 10.0)
  (`KismetSystemLibrary.PrintString` "CameraRig:  \n" true true (struct :`R` 1.0 :`B` 0.942668 :`A` 1.0) 10.0))

(fn `SetCurrentCameraRig`
  (params (CurrentCameraRig :type "/Game/PluginAssets/CameraRig/Blueprint/Rigs/Base/BP_CameraRig_Base Object Reference"))
  (set `self.CurrentCameraRig` CurrentCameraRig)
  (return))

(fn `SetGlobalFocusSettings`
  (params (Global_FocusSettings :type "/Game/PluginAssets/CameraRig/Structs/S_CameraRig_FocusSettings Structure"))
  (set `self.Global_FocusSettings` Global_FocusSettings)
  (return))

(fn `SetGlobalTrackingSettings`
  (params (Global_LookatTrackingSettings :type "CameraLookatTrackingSettings Structure"))
  (set `self.Global_LookatTrackingSettings` Global_LookatTrackingSettings)
  (for _array_element (`self.GetAllCameraRigRefs`)
    (`/Game/PluginAssets/CameraRig/Blueprint/Rigs/Base/BP_CameraRig_Base.UpdateCurrentTrackingSettings` _array_element))
  (return))

(fn `SetLocalFocusSettings`
  (params (CameraRig :type "/Game/PluginAssets/CameraRig/Blueprint/Rigs/Base/BP_CameraRig_Base Object Reference") (NewFocusSettings :type "/Game/PluginAssets/CameraRig/Structs/S_CameraRig_FocusSettings Structure"))
  (`/Game/PluginAssets/CameraRig/Blueprint/Rigs/Base/BP_CameraRig_Base.SetLocalFocusSettings` CameraRig NewFocusSettings)
  (return))

(fn `SetLocalTrackingSettings`
  (params (CameraRig :type "/Game/PluginAssets/CameraRig/Blueprint/Rigs/Base/BP_CameraRig_Base Object Reference") (NewLookatTrackingSettings :type "CameraLookatTrackingSettings Structure"))
  (`/Game/PluginAssets/CameraRig/Blueprint/Rigs/Base/BP_CameraRig_Base.SetLocalTrackingSettings` CameraRig NewLookatTrackingSettings)
  (return))

(fn `SetRailSettings`
  (params (CameraRig :type "/Game/PluginAssets/CameraRig/Blueprint/Rigs/Base/BP_CameraRig_Base Object Reference") (CameraRail_Settings :type "/Game/PluginAssets/CameraRig/Structs/S_CameraRail_Settings Structure"))
  (locals (L_CameraRig :type "/Game/PluginAssets/CameraRig/Blueprint/Rigs/Base/BP_CameraRig_Base Object Reference") (L_CameraRailSettings :type "/Game/PluginAssets/CameraRig/Structs/S_CameraRail_Settings Structure"))
  (set `local.L_CameraRig` CameraRig)
  (set `local.L_CameraRailSettings` CameraRail_Settings)
  (`/Engine/EditorBlueprintResources/StandardMacros.IsValid` (`local.L_CameraRig`)
    (:`Is Valid`
      (`/Game/PluginAssets/CameraRig/Blueprint/Rigs/Base/BP_CameraRig_Base.SetRailSettings` (`local.L_CameraRig`) (`local.L_CameraRailSettings`)))))

(fn `SetRigChangingState`
  (params (`RigChanging?` :type Boolean))
  (set `self.OnRigChanging?` `RigChanging?`)
  (return))

(fn `SetStartBlendSettings`
  (params (CameraRig :type "/Game/PluginAssets/CameraRig/Blueprint/Rigs/Base/BP_CameraRig_Base Object Reference") (NewBlendTime :type "Float (double-precision)") (StartBlendFunction :type "EViewTargetBlendFunction Enum" :default "VTBlend_Linear"))
  (locals (L_CameraRig :type "/Game/PluginAssets/CameraRig/Blueprint/Rigs/Base/BP_CameraRig_Base Object Reference") (L_CurrentSwitchSettings :type "/Game/PluginAssets/CameraRig/Structs/S_CameraSwitchSettings Structure"))
  (bind _output_get (set `local.L_CameraRig` CameraRig))
  (set `/Game/PluginAssets/CameraRig/Blueprint/Rigs/Base/BP_CameraRig_Base.StartBlendTime` NewBlendTime _output_get)
  (set `/Game/PluginAssets/CameraRig/Blueprint/Rigs/Base/BP_CameraRig_Base.StartBlendFunction` StartBlendFunction _output_get)
  (return))

(fn `SetSwitchSettings`
  (params (CameraRig :type "/Game/PluginAssets/CameraRig/Blueprint/Rigs/Base/BP_CameraRig_Base Object Reference") (CurrentSwitchSettings :type "/Game/PluginAssets/CameraRig/Structs/S_CameraSwitchSettings Structure"))
  (locals (L_CameraRig :type "/Game/PluginAssets/CameraRig/Blueprint/Rigs/Base/BP_CameraRig_Base Object Reference") (L_CurrentSwitchSettings :type "/Game/PluginAssets/CameraRig/Structs/S_CameraSwitchSettings Structure"))
  (set `local.L_CameraRig` CameraRig)
  (set `local.L_CurrentSwitchSettings` CurrentSwitchSettings)
  (`/Engine/EditorBlueprintResources/StandardMacros.IsValid` (`local.L_CameraRig`)
    (:`Is Valid`
      (`/Game/PluginAssets/CameraRig/Blueprint/Rigs/Base/BP_CameraRig_Base.SetSwitchSettings` (`local.L_CameraRig`) (`local.L_CurrentSwitchSettings`)))))

(fn `StartCollisionTests_Intervall`
  (params (CameraRig :type "/Game/PluginAssets/CameraRig/Blueprint/Rigs/Base/BP_CameraRig_Base Object Reference") (`ChangeSettings?` :type Boolean) (IntervallSettings :type "/Game/PluginAssets/CameraRig/Structs/S_CameraRig_IntervallTest_Settings Structure"))
  (locals (L_CameraRig :type "/Game/PluginAssets/CameraRig/Blueprint/Rigs/Base/BP_CameraRig_Base Object Reference") (L_ChangeSettings :type Boolean) (L_IntervallSettings :type "/Game/PluginAssets/CameraRig/Structs/S_CameraRig_IntervallTest_Settings Structure"))
  (set `local.L_CameraRig` CameraRig)
  (set `local.L_ChangeSettings` `ChangeSettings?`)
  (set `local.L_IntervallSettings` IntervallSettings)
  (if (`local.L_ChangeSettings`)
    (`/Game/PluginAssets/CameraRig/Blueprint/Rigs/Base/BP_CameraRig_Base.SetIntervallTest_Settings` (`local.L_CameraRig`) (`local.L_IntervallSettings`))
    (`/Game/PluginAssets/CameraRig/Blueprint/Rigs/Base/BP_CameraRig_Base.SetCollisionTest_IntervallTimer` (`local.L_CameraRig`))
    (else
      (`/Game/PluginAssets/CameraRig/Blueprint/Rigs/Base/BP_CameraRig_Base.SetCollisionTest_IntervallTimer` (`local.L_CameraRig`)))))

(fn `StopCollisionTests_Intervall`
  (params (CameraRig :type "/Game/PluginAssets/CameraRig/Blueprint/Rigs/Base/BP_CameraRig_Base Object Reference"))
  (locals (L_CameraRig :type "/Game/PluginAssets/CameraRig/Blueprint/Rigs/Base/BP_CameraRig_Base Object Reference"))
  (bind _output_get (set `local.L_CameraRig` CameraRig))
  (`/Game/PluginAssets/CameraRig/Blueprint/Rigs/Base/BP_CameraRig_Base.StopCollisionTest_IntervallTimer` _output_get))

(fn `TriggerCameraRigByName`
  (params (CameraRigName :type Text) (Type :type "/Game/PluginAssets/CameraRig/Enums/E_Camspot_Type Enum" :default "NewEnumerator0") (TriggerSpot_Index :type Integer))
  (locals (L_RigName :type Text))
  (bind _output_get (set `local.L_RigName` CameraRigName))
  (bind (_found_ _camerarig) (`self.GetCameraRigByName` _output_get))
  (if _found_
    (if (not (== (`self.CurrentCameraRig`) _camerarig))
      (`/Engine/EditorBlueprintResources/StandardMacros.IsValid` (`self.CurrentCameraRig`)
        (:`Is Not Valid`
          _)))
    (`self.SetCurrentCameraRig` _camerarig)
    (`/Game/PluginAssets/CameraRig/Blueprint/Rigs/Base/BP_CameraRig_Base.CE_TriggerCamera` _camerarig Type TriggerSpot_Index false)
    (else
      (`self.PrintString_Debug` "NewEnumerator1" (`KismetStringLibrary.Concat_StrStr` "Cant trigger rig! \n \nName is not valid! \n" "Name: " (`KismetTextLibrary.Conv_TextToString` (`local.L_RigName`)))))))

(fn `TriggerCameraRigByRef`
  (params (CameraRig :type "/Game/PluginAssets/CameraRig/Blueprint/Rigs/Base/BP_CameraRig_Base Object Reference") (Type :type "/Game/PluginAssets/CameraRig/Enums/E_Camspot_Type Enum" :default "NewEnumerator0") (TriggerSpot_Index :type Integer))
  (`/Engine/EditorBlueprintResources/StandardMacros.IsValid` CameraRig
    (:`Is Valid`
      (`self.SetCurrentCameraRig` CameraRig)
      (`/Game/PluginAssets/CameraRig/Blueprint/Rigs/Base/BP_CameraRig_Base.CE_TriggerCamera` CameraRig Type TriggerSpot_Index false))))

(fn `UpdateTrackingActor`
  (params (`Enable Look at Tracking` :type Boolean :default true) (`Actor to Track` :type "Actor Soft Object Reference") (`Relative Offset` :type "Vector Structure") (`NewSpeed?` :type Boolean) (`Look at Tracking Interp Speed` :type "Float (double-precision)" :default 0.0))
  (bind _structout (setmembers `CameraLookatTrackingSettings` :`StructRef` (`self.GetGlobalTrackingSettings`) :`bEnableLookAtTracking` `Enable Look at Tracking` :`LookAtTrackingInterpSpeed` (select `bool` `NewSpeed?` :`false` (`.LookAtTrackingInterpSpeed` (break `CameraLookatTrackingSettings` (`self.GetGlobalTrackingSettings`))) :`true` `Look at Tracking Interp Speed` :!type "Float (double-precision)") :`ActorToTrack` `Actor to Track` :`RelativeOffset` `Relative Offset`))
  (`self.SetGlobalTrackingSettings` _structout))