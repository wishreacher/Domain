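; BP_CameraRig_01 is a camera rig variant that supplies its own set of camera rails and spots.
; CreateCameraRails returns two spline components as the rails, and CreateCameraSpots returns two arrow components as the spots.
; It holds no other logic of its own: the construction script only calls the parent, and the event graph is disabled.
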(fn `CreateCameraRails`
  (returns (Array :type "Array of SplineComponent Object Reference"))
  (return (`|MakeArray` (`self.Spline`) (`self.Spline1`))))

(fn `CreateCameraSpots`
  (returns (Array :type "Array of SceneComponent Object Reference"))
  (return (`|MakeArray` (`self.Arrow`) (`self.Arrow1`) :!type "SceneComponent Object Reference")))

(fn `UserConstructionScript`
  (`parent.UserConstructionScript`))